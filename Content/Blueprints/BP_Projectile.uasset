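; BP_Projectile is a physics-driven projectile actor with a function to launch it along its forward vector.
; LaunchAmmo adds a fixed impulse to the SMProjectile component as a velocity change, so the launch speed ignores mass.
; PrintAmmoName prints the actor's display name with a spawn message for debugging.
; The event graph and construction script do nothing, so neither function is called within this Blueprint.
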(event EventBeginPlay)

(event Collision|EventActorBeginOverlap
  (params (OtherActor :type Actor%20Object%20Reference)))

(event EventTick
  (params (DeltaSeconds :type Float%20%28single-precision%29)))

(fn ConstructionScript)

(fn PrintAmmoName
  (Development|PrintString (Utilities|String|Append (Utilities|GetDisplayName self) " has Spawned")))

(fn LaunchAmmo
  (bind _self self)
  (Physics|AddImpulse (Variables|BP_Projectile_C|GetSM_Projectile _self) (* (Transformation|GetActorForwardVector _self) 4e+03) "None" true))