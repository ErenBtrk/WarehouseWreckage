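; Player pawn for the Warehouse Wreckage game that fires limited-ammo projectiles and restarts the level when ammo runs out.
; Left click spawns and launches a BP_Projectile from the pawn along the control rotation, then decrements and prints AmmoCount.
; On an empty click, a DoOnce-guarded Timeline serves as the restart countdown, printing near-whole-second values before reopening the current level.
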(event EventBeginPlay
  (CallFunction|PrintWelcomeMessage))

(event Collision|EventActorBeginOverlap
  (params (OtherActor :type Actor%20Object%20Reference)))

(event Input|MouseEvents|LeftMouseButton
  (params (Key :type Key%20Structure :default "None"))
  (:Pressed
    (if (CallFunction|HasAmmo (Variables|Default|GetAmmoCount))
      (CallFunction|SpawnAmmo)
      (CallFunction|DecreaseAmmo)
      (CallFunction|PrintAmmo)
      (else
        (Utilities|FlowControl|DoOnce false
          (:Completed
            (Development|PrintString "Out of Ammo, restarting in 5 seconds")
            (bind _newtrack_0 (Timeline|Timeline PlayFromStart)
              (:Update
                (CallFunction|CheckDecimalPart _newtrack_0))
              (:Finished
                (CallFunction|RestartLevel)))))))))

(fn ConstructionScript)

(fn SpawnAmmo
  (bind _returnvalue (Game|SpawnActorfromClass "/Game/Blueprints/BP_Projectile.BP_Projectile_C" (Math|Transform|MakeTransform (Transformation|GetActorLocation) (Pawn|GetControlRotation :!class /Script/Engine.Pawn) "1.000000,1.000000,1.000000") "Undefined" 0 0))
  (Default|PrintAmmoName _returnvalue)
  (Default|LaunchAmmo _returnvalue))

(fn PrintAmmo
  (Development|PrintString (Utilities|String|Append (Utilities|String|ToString(Integer) (Variables|Default|GetAmmoCount)) " Ammo Left")))

(fn DecreaseAmmo
  (Math|Integer|DecrementInt (Variables|Default|GetAmmoCount)))

(fn PrintWelcomeMessage
  (Development|PrintString "Welcome to the Warehose Wreckage Game"))

(fn HasAmmo
  (params (CurrentAmmo :type Integer))
  (return (> CurrentAmmo 0)))

(fn RestartLevel
  (bind _returnvalue (Game|GetCurrentLevelName true))
  (Game|OpenLevel(byName) (Utilities|String|StringToName _returnvalue)))

(fn CheckDecimalPart
  (params (FloatNum :type Float%20%28double-precision%29))
  (bind _returnvalue (Math|Float|Floor FloatNum))
  (if (Math|Float|NearlyEqual(Float) (- FloatNum (Math|Conversions|ToFloat(Integer) _returnvalue)) 0.0 0.001)
    (Development|PrintString (Utilities|String|Append "Restarting in " (Utilities|String|ToString(Integer) _returnvalue) " Seconds"))
    (return)))